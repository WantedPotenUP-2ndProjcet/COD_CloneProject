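; BP_Aircraft is an allied aircraft actor that flies a one-way curved path over about 15 seconds.
; Tick advances a clamped Timer and evaluates a cubic Bézier from InitLoc to Target3 through nested lerps, using Target1 and Target2 as control points.
; Each step also orients the aircraft along its movement direction with a fixed roll offset for banking.
; BeginPlay and overlap are empty, and the airstrike sound nodes are disconnected.
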(event `self.ReceiveBeginPlay`)

(event `self.ReceiveTick`
  (params (DeltaSeconds :type "Float (single-precision)"))
  (bind _returnvalue (`self.K2_GetActorLocation` (`self.Target1`)))
  (bind _returnvalue_2 (`self.K2_GetActorLocation` (`self.Target2`)))
  (bind _output_get (set `self.Timer` (`KismetMathLibrary.FClamp` (+ (/ DeltaSeconds 15.0) (`self.Timer`)))))
  (bind _returnvalue_3 (`KismetMathLibrary.VLerp` _returnvalue _returnvalue_2 _output_get))
  (bind _returnvalue_4 (`KismetMathLibrary.VLerp` (`KismetMathLibrary.VLerp` (`KismetMathLibrary.VLerp` (`self.InitLoc`) _returnvalue _output_get) _returnvalue_3 _output_get) (`KismetMathLibrary.VLerp` _returnvalue_3 (`KismetMathLibrary.VLerp` _returnvalue_2 (`self.K2_GetActorLocation` (`self.Target3`)) _output_get) _output_get) _output_get))
  (`self.K2_SetActorLocationAndRotation` _returnvalue_4 (`KismetMathLibrary.MakeRotator` (+ -50.0 (.roll (`KismetMathLibrary.Conv_VectorToRotator` (- _returnvalue_4 (`self.K2_GetActorLocation`))))) (.pitch (`KismetMathLibrary.Conv_VectorToRotator` (- _returnvalue_4 (`self.K2_GetActorLocation`)))) (.yaw (`KismetMathLibrary.Conv_VectorToRotator` (- _returnvalue_4 (`self.K2_GetActorLocation`)))))))

(fn `UserConstructionScript`)