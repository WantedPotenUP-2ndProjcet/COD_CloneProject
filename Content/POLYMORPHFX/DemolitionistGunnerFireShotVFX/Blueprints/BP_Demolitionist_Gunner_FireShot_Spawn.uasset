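; Spawner actor for the Demolitionist Gunner FireShot VFX that plays a repeating, timed firing sequence from BeginPlay.
; One branch attaches a mark and four muzzle flash Niagara systems to the Muzzleflash component.
; A parallel branch spawns projectile actors at the Projectile component's transform on matching delays, three of one type then a different final one.
; Both branches meet at a shared delay that calls Success to restart the loop.
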(event `Success`
  (bind _muzzleflash (`self.Muzzleflash`))
  (bind _returnvalue (`SceneComponent.K2_GetComponentToWorld` (`self.Projectile`)))
  (`|ExecutionSequence` :!label _label
    (:`then_0`
      ;[1 0.7493 0.7394] Mark
      (`NiagaraFunctionLibrary.SpawnSystemAttached` "/Game/POLYMORPHFX/DemolitionistGunnerFireShotVFX/Niagara/NS_Demolitionist_Gunner_FireShot_Mark.NS_Demolitionist_Gunner_FireShot_Mark" _muzzleflash "None" (0.0 0.0 0.0) (struct) "KeepRelativeOffset")
      ;[0.7186 0.7607 1] Muzzleflash
      (`NiagaraFunctionLibrary.SpawnSystemAttached` "/Game/POLYMORPHFX/DemolitionistGunnerFireShotVFX/Niagara/NS_Demolitionist_Gunner_FireShot_Muzzleflash_01.NS_Demolitionist_Gunner_FireShot_Muzzleflash_01" _muzzleflash "None" (0.0 0.0 0.0) (struct) "KeepRelativeOffset")
      (`KismetSystemLibrary.Delay` 0.8)
      (`NiagaraFunctionLibrary.SpawnSystemAttached` "/Game/POLYMORPHFX/DemolitionistGunnerFireShotVFX/Niagara/NS_Demolitionist_Gunner_FireShot_Muzzleflash_01.NS_Demolitionist_Gunner_FireShot_Muzzleflash_01" _muzzleflash "None" (0.0 0.0 0.0) (struct) "KeepRelativeOffset")
      (`KismetSystemLibrary.Delay` 0.72)
      (`NiagaraFunctionLibrary.SpawnSystemAttached` "/Game/POLYMORPHFX/DemolitionistGunnerFireShotVFX/Niagara/NS_Demolitionist_Gunner_FireShot_Muzzleflash_01.NS_Demolitionist_Gunner_FireShot_Muzzleflash_01" _muzzleflash "None" (0.0 0.0 0.0) (struct) "KeepRelativeOffset")
      (`KismetSystemLibrary.Delay` 1.66)
      (`NiagaraFunctionLibrary.SpawnSystemAttached` "/Game/POLYMORPHFX/DemolitionistGunnerFireShotVFX/Niagara/NS_Demolitionist_Gunner_FireShot_Muzzleflash_02.NS_Demolitionist_Gunner_FireShot_Muzzleflash_02" _muzzleflash "None" (0.0 0.0 0.0) (struct) "KeepRelativeOffset"))
    (:`then_1`
      ;[0.7713 1 0.7716 0.5] Projectiles
      (`|SpawnActorFromClass` "/Game/POLYMORPHFX/DemolitionistGunnerFireShotVFX/Blueprints/BP_Demolitionist_Gunner_FireShot_Projectile_01.BP_Demolitionist_Gunner_FireShot_Projectile_01_C" _returnvalue "Undefined" "MultiplyWithRoot" null null)
      (`KismetSystemLibrary.Delay` 0.8)
      (`|SpawnActorFromClass` "/Game/POLYMORPHFX/DemolitionistGunnerFireShotVFX/Blueprints/BP_Demolitionist_Gunner_FireShot_Projectile_01.BP_Demolitionist_Gunner_FireShot_Projectile_01_C" _returnvalue "Undefined" "MultiplyWithRoot" null null)
      (`KismetSystemLibrary.Delay` 0.72)
      (`|SpawnActorFromClass` "/Game/POLYMORPHFX/DemolitionistGunnerFireShotVFX/Blueprints/BP_Demolitionist_Gunner_FireShot_Projectile_01.BP_Demolitionist_Gunner_FireShot_Projectile_01_C" _returnvalue "Undefined" "MultiplyWithRoot" null null)
      (`KismetSystemLibrary.Delay` 1.66)
      (`|SpawnActorFromClass` "/Game/POLYMORPHFX/DemolitionistGunnerFireShotVFX/Blueprints/BP_Demolitionist_Gunner_FireShot_Projectile_02.BP_Demolitionist_Gunner_FireShot_Projectile_02_C" _returnvalue "Undefined" "MultiplyWithRoot" null null)))
  (`KismetSystemLibrary.Delay` 2.0)
  (`self.Success`))

(event `self.ReceiveBeginPlay`
  (goto _label))

(fn `UserConstructionScript`)