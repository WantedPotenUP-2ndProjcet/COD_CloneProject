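; BP_TestActor is a test hazard that fires projectiles on a timer and triggers player death on contact.
; Tick accumulates delta time and, each time MaxTime is reached, resets it and spawns a BP_TestActorBullet at the BulletSpawnPoint transform.
; Any overlap with its Cube calls PlayerDeadEvent on BP_PlayerTestGameMode, without checking which actor overlapped.
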(event `self.ReceiveTick`
  (params (DeltaSeconds :type "Float (single-precision)"))
  (bind _output_get (set `self.CurrentTime` (+ DeltaSeconds (`self.CurrentTime`))))
  (if (>= _output_get (`self.MaxTime`))
    (set `self.CurrentTime` 0.0)
    (`|SpawnActorFromClass` "/Game/MainPlayer/Weapon/Blueprints/Bullets/BP_TestActorBullet.BP_TestActorBullet_C" (`SceneComponent.K2_GetComponentToWorld` (`self.BulletSpawnPoint`)) "Undefined" "MultiplyWithRoot" null null)))

(event `self.Cube.OnComponentBeginOverlap`
  (params (OverlappedComponent :type "PrimitiveComponent Object Reference") (OtherActor :type "Actor Object Reference") (OtherComp :type "PrimitiveComponent Object Reference") (OtherBodyIndex :type Integer) (bFromSweep :type Boolean) (SweepResult :type "HitResult Structure (by ref)"))
  (bind _asbp_player_test_game_mode (cast `/Game/MainPlayer/Map/BP_PlayerTestGameMode` (`GameplayStatics.GetGameMode`)))
  (`/Game/MainPlayer/Map/BP_PlayerTestGameMode.PlayerDeadEvent` _asbp_player_test_game_mode))

(fn `UserConstructionScript`)