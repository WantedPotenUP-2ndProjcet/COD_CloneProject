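; BP_TestBullet is a test projectile actor that flies straight and damages whatever it overlaps.
; Each tick it moves along its forward vector by Speed scaled by delta time, using a non-swept location set.
; On actor overlap it prints its owner's name and applies fixed damage to the other actor, with the owner as damage causer.
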(event `self.ReceiveActorBeginOverlap`
  (params (OtherActor :type "Actor Object Reference"))
  (bind _returnvalue (`self.GetOwner`))
  (`KismetSystemLibrary.PrintString` (`KismetSystemLibrary.GetObjectName` _returnvalue))
  (`GameplayStatics.ApplyDamage` OtherActor 10.0 null _returnvalue))

(event `self.ReceiveTick`
  (params (DeltaSeconds :type "Float (single-precision)"))
  (`self.K2_SetActorLocation` (+ (* DeltaSeconds (* (`self.Speed`) (`self.GetActorForwardVector`))) (`self.K2_GetActorLocation`))))

(fn `UserConstructionScript`)