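; Game mode for a player test map that ends the run as a clear after a 45-second survival timer, or as a loss on player death.
; BeginPlay sets game-only input and pre-creates the clear and death widgets.
; Tick accumulates time and fires GameClearEvent past the limit; PlayerDeadEvent has no caller in this graph.
; Both events remove the player HUD, show their widget, switch to UI-only input with cursor, and pause.
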(event `self.ReceiveBeginPlay`
  (bind _returnvalue (`GameplayStatics.GetPlayerController` 0))
  (set `PlayerController.bShowMouseCursor` false _returnvalue)
  (`WidgetBlueprintLibrary.SetInputMode_GameOnly` _returnvalue)
  (bind _returnvalue_2 (`|CreateWidget` "/Game/MainPlayer/UI/WBP_ClearGame.WBP_ClearGame_C" _returnvalue))
  (set `self.ClearGameUI` _returnvalue_2)
  (bind _returnvalue_3 (`|CreateWidget` "/Game/MainPlayer/UI/WBP_Death.WBP_Death_C" _returnvalue))
  (set `self.DeathUI` _returnvalue_3))

(event `self.ReceiveTick`
  (params (DeltaSeconds :type "Float (single-precision)"))
  (bind _output_get (set `self.CurrentTime` (+ DeltaSeconds (`self.CurrentTime`))))
  (if (> _output_get 45.0)
    (`self.GameClearEvent`)))

(event `GameClearEvent`
  (bind _returnvalue (`GameplayStatics.GetPlayerController` 0))
  (bind _asbp_main_player_character (cast `/Game/MainPlayer/Character/BP_MainPlayerCharacter` (`GameplayStatics.GetPlayerPawn` 0)))
  (`Widget.RemoveFromParent` (`/Game/MainPlayer/Character/BP_MainPlayerCharacter.PlayerUI` _asbp_main_player_character))
  (`UserWidget.AddToViewport` (`self.ClearGameUI`) 0)
  (set `PlayerController.bShowMouseCursor` true _returnvalue)
  (`WidgetBlueprintLibrary.SetInputMode_UIOnlyEx` _returnvalue (`self.ClearGameUI`))
  (`GameplayStatics.SetGamePaused` true))

(event `PlayerDeadEvent`
  (bind _returnvalue (`GameplayStatics.GetPlayerController` 0))
  (bind _asbp_main_player_character (cast `/Game/MainPlayer/Character/BP_MainPlayerCharacter` (`GameplayStatics.GetPlayerPawn` 0)))
  (`Widget.RemoveFromParent` (`/Game/MainPlayer/Character/BP_MainPlayerCharacter.PlayerUI` _asbp_main_player_character))
  (`UserWidget.AddToViewport` (`self.DeathUI`) 0)
  (set `PlayerController.bShowMouseCursor` true _returnvalue)
  (`WidgetBlueprintLibrary.SetInputMode_UIOnlyEx` _returnvalue (`self.DeathUI`))
  (`GameplayStatics.SetGamePaused` true))

(fn `UserConstructionScript`)