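; Base weapon Blueprint for the main player, handling firing, magazine count and bullet spawning.
; On BeginPlay it loads its stats and bullet class from a data table row and caches the player's AttackComponent.
; FireBullet shoots once, then loops on an RPM timer for automatic weapons until stopped or empty.
; Each shot traces from screen center, randomizes direction within the AttackComponent's aim cone, spawns the bullet and triggers the fire animation.
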(event `self.ReceiveBeginPlay`
  (bind (_datatable _rowname) (break `DataTableRowHandle` (`self.WeaponData`)))
  (bind _asbp_main_player_character (cast `/Game/MainPlayer/Character/BP_MainPlayerCharacter` (`GameplayStatics.GetPlayerPawn` 0)))
  (set `self.AttackComponent` (`/Game/MainPlayer/Character/BP_MainPlayerCharacter.AttackComponent` _asbp_main_player_character))
  (bind _returnvalue (`|GetDataTableRow` _datatable _rowname)
    (:`then`
      (bind (_name _damage _rpm _maximumrange _validmaxrange _bcanauto _recoil _magazinesize _pickupweapon _equipmentweapon _bullet) (break `/Game/MainPlayer/Data/Weapon/F_WeaponData` _returnvalue))
      (set `self.RPM` _rpm)
      (set `self.MaxRange` _maximumrange)
      (set `self.bCanAuto` _bcanauto)
      (set `self.Recoil` _recoil)
      (set `self.RemainRounds` _magazinesize)
      (set `self.BulletClass` _bullet))))

(event `SetTargetVectorForBullet`
  (params (BulletDirection :type "Vector Structure"))
  (`SceneComponent.K2_SetWorldRotation` (`self.BulletSpawnPoint`) (`KismetMathLibrary.Conv_VectorToRotator` BulletDirection) false false))

(fn `FireBullet`
  (bind _returnvalue (/ 60.0 (`self.RPM`)))
  ; 일단 한 발 발사
  (`self.SpawnBullet`)
  ; 연사 가능여부 확인
  (if (`self.bCanAuto`)
    ; rpm마다 fire
    (bind _returnvalue_2 (`KismetSystemLibrary.K2_SetTimer` null "SpawnBullet" _returnvalue true false _returnvalue))
    (set `self.FireTimerHandle` _returnvalue_2)))

(fn `GetShootTargetLocation`
  (returns (TargetLocation :type "Vector Structure"))
  (bind (_worldposition _worlddirection) (`GameplayStatics.DeprojectScreenToWorld` (`GameplayStatics.GetPlayerController` 0) (/ (`WidgetLayoutLibrary.GetViewportSize`) 2.0)))
  (bind _returnvalue (+ _worldposition (* _worlddirection (`self.MaxRange`))))
  (bind (_outhit _returnvalue_2) (`KismetSystemLibrary.LineTraceSingle` _worldposition _returnvalue "TraceTypeQuery1"))
  (if _returnvalue_2
    (return (`.ImpactPoint` (`GameplayStatics.BreakHitResult` _outhit)))
    (else
      (return _returnvalue))))

(fn `SpawnBullet`
  (bind _bulletclass (`self.BulletClass`))
  ; Check Remaining Rounds
  (if (> (`self.RemainRounds`) 0)
    ; Weapon Data에서 가져온 총알 정보로 총알 생성
    (if (`KismetSystemLibrary.IsValidClass` _bulletclass)
      ; 총알 방향 조정
      (bind _targetlocation (`self.GetShootTargetLocation`))
      (bind _bulletdirection (`self.SpreadBullet` _targetlocation))
      (`self.SetTargetVectorForBullet` _bulletdirection)
      (`|SpawnActorFromClass` _bulletclass (`SceneComponent.K2_GetComponentToWorld` (`self.BulletSpawnPoint`)) "Undefined" "MultiplyWithRoot" null null)
      (bind _asbp_main_player_character (cast `/Game/MainPlayer/Character/BP_MainPlayerCharacter` (`GameplayStatics.GetPlayerPawn` 0)))
      (`/Game/MainPlayer/Character/AttackComponent.FireAnimation` (`/Game/MainPlayer/Character/BP_MainPlayerCharacter.AttackComponent` _asbp_main_player_character))
      ; 남은 총탄 수 저장
      (bind _output_get (set `self.RemainRounds` (- (`self.RemainRounds`) 1)))
      (`KismetSystemLibrary.PrintString` (`KismetStringLibrary.Conv_IntToString` _output_get)))
    (else
      (`KismetSystemLibrary.K2_ClearAndInvalidateTimerHandle` (`self.FireTimerHandle`)))))

(fn `SpreadBullet`
  (params (TargetLocation :type "Vector Structure"))
  (returns (BulletDirection :type "Vector Structure"))
  (return (`KismetMathLibrary.RandomUnitVectorInConeInDegrees` (`KismetMathLibrary.Normal` (- TargetLocation (`SceneComponent.K2_GetComponentLocation` (`self.BulletSpawnPoint`)))) (`/Game/MainPlayer/Character/AttackComponent.MaxAimRange` (`self.AttackComponent`)))))

(fn `StopFire`
  (`KismetSystemLibrary.K2_ClearAndInvalidateTimerHandle` (`self.FireTimerHandle`)))

(fn `UserConstructionScript`)