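; BP_PickUpWeaponBase is a base actor for weapon pickups that the main player can collect.
; On BeginPlay it reads the weapon's name and image from a data table row.
; Its collision overlap shows or hides the player UI's pickup panel with that info.
; The PickUp event looks up the row again, passes the equipment weapon to the player's AttackComponent, then destroys the pickup.
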(event `self.ReceiveBeginPlay`
  (bind (_datatable _rowname) (break `DataTableRowHandle` (`self.WeaponData`)))
  (bind _returnvalue (`|GetDataTableRow` _datatable _rowname)
    (:`then`
      (bind ((`Name_5_46E02F5F44D6D4705BF34CAA35193D77` _name) (`WeaponImage_51_7D3C716944D1D88EB9C958A32D650076` _weaponimage)) (break `/Game/MainPlayer/Data/Weapon/F_WeaponData` _returnvalue))
      (set `self.WeaponName` (`KismetTextLibrary.Conv_NameToText` _name))
      (set `self.WeaponImage` _weaponimage))))

(event `/Game/MainPlayer/Weapon/Blueprints/BP_InteractWeapon.PickUp`
  (params (MainPlayer :type "/Game/MainPlayer/Character/BP_MainPlayerCharacter Object Reference"))
  (bind (_datatable _rowname) (break `DataTableRowHandle` (`self.WeaponData`)))
  (bind _returnvalue (`|GetDataTableRow` _datatable _rowname)
    (:`then`
      (`/Game/MainPlayer/Character/AttackComponent.PickUpWeapon` (`/Game/MainPlayer/Character/BP_MainPlayerCharacter.AttackComponent` MainPlayer) (`.EquipmentWeapon_30_1B5697BF47FD131967E395B99D95854B` (break `/Game/MainPlayer/Data/Weapon/F_WeaponData` _returnvalue)))
      (`self.K2_DestroyActor`))))

(event `self.PickUpCollision.OnComponentBeginOverlap`
  (params (OverlappedComponent :type "PrimitiveComponent Object Reference") (OtherActor :type "Actor Object Reference") (OtherComp :type "PrimitiveComponent Object Reference") (OtherBodyIndex :type Integer) (bFromSweep :type Boolean) (SweepResult :type "HitResult Structure (by ref)"))
  (bind _asbp_main_player_character (cast `/Game/MainPlayer/Character/BP_MainPlayerCharacter` OtherActor))
  (`/Game/MainPlayer/UI/WBP_MainPlayer.ShowPickUpPanel` (`/Game/MainPlayer/Character/BP_MainPlayerCharacter.PlayerUI` _asbp_main_player_character) (`self.WeaponImage`) (`self.WeaponName`)))

(event `self.PickUpCollision.OnComponentEndOverlap`
  (params (OverlappedComponent :type "PrimitiveComponent Object Reference") (OtherActor :type "Actor Object Reference") (OtherComp :type "PrimitiveComponent Object Reference") (OtherBodyIndex :type Integer))
  (bind _asbp_main_player_character (cast `/Game/MainPlayer/Character/BP_MainPlayerCharacter` OtherActor))
  (`/Game/MainPlayer/UI/WBP_MainPlayer.ShowOffPickUpPanel` (`/Game/MainPlayer/Character/BP_MainPlayerCharacter.PlayerUI` _asbp_main_player_character)))

(fn `UserConstructionScript`)