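; BP_EnemyMortar is an enemy that crouches into cover, rises to shoot at the player, and dies from damage.
; AnyDamage reduces health, enables mesh ragdoll physics at zero, and destroys the actor after a timer.
; Cover and Fire events, apparently driven through an interface, handle crouching and delayed shooting.
; Shoot spawns a projectile aimed straight at the player's current location, with muzzle flash and sound.
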(event `self.ReceiveBeginPlay`)

(event `self.ReceiveTick`
  (params (DeltaSeconds :type "Float (single-precision)")))

(event `self.ReceiveAnyDamage`
  (params (Damage :type "Float (single-precision)") (DamageType :type "DamageType Object Reference") (InstigatedBy :type "Controller Object Reference") (DamageCauser :type "Actor Object Reference"))
  ; OnDamaged > Ragdoll > Destroy
  (bind _output_get (set `self.CurrentHealth` (- (`self.CurrentHealth`) Damage)))
  (if (<= _output_get 0.0)
    (set `self.IsDead` true)
    (`PrimitiveComponent.SetSimulatePhysics` (`self.Mesh`) true)
    (`KismetSystemLibrary.K2_SetTimerDelegate` (delegate `Dead`) 5.0)))

(event `Dead`
  ; OnDamaged > Ragdoll > Destroy
  (`self.K2_DestroyActor`))

(event `self.Cover`
  ; Cover / UnCover BPI 연동
  (`self.Crouch`))

(event `Shoot`
  (bind _bulletfirepoint (`self.BulletFirePoint`))
  (bind _returnvalue_location (`KismetMathLibrary.BreakTransform` (`SceneComponent.K2_GetComponentToWorld` _bulletfirepoint)))
  (bind _returnvalue (`KismetMathLibrary.FindLookAtRotation` _returnvalue_location (`self.K2_GetActorLocation` (`GameplayStatics.GetPlayerCharacter` 0))))
  ; Shoot Event
  (`|SpawnActorFromClass` "/Game/Huxley/EnemyAI/BP_EnemyProjectile.BP_EnemyProjectile_C" (`KismetMathLibrary.MakeTransform` _returnvalue_location _returnvalue) "Undefined" "MultiplyWithRoot" null null)
  (`NiagaraFunctionLibrary.SpawnSystemAtLocation` "/Game/POLYMORPHFX/DemolitionistGunnerFireShotVFX/Niagara/NS_Demolitionist_Gunner_FireShot_Muzzleflash_01.NS_Demolitionist_Gunner_FireShot_Muzzleflash_01" _returnvalue_location _returnvalue)
  (`GameplayStatics.PlaySoundAtLocation` "/Game/FPWeapon/Audio/FirstPersonTemplateWeaponFire02.FirstPersonTemplateWeaponFire02" (`SceneComponent.K2_GetComponentLocation` _bulletfirepoint) (struct) 1.0 1.0 0.0 null null null null))

(event `self.Fire`
  ; Cover / UnCover BPI 연동
  (`self.UnCrouch`)
  (`KismetSystemLibrary.Delay` 1.0)
  (`self.Shoot`))

(fn `UserConstructionScript`)