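; Enemy AI character Blueprint that crouches for cover and stands to fire short projectile bursts at its target.
; Fire uncrouches, waits, then loops Shoot on a timer for a random shot count, each shot re-reading TargetActor from the Blackboard.
; Shots spawn BP_EnemyProjectile with random spread, muzzle flash and a random sound.
; Damage reduces health; at zero the mesh ragdolls and the actor is destroyed after a delay.
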(event `self.ReceiveTick`
  (params (DeltaSeconds :type "Float (single-precision)")))

(event `self.ReceiveAnyDamage`
  (params (Damage :type "Float (single-precision)") (DamageType :type "DamageType Object Reference") (InstigatedBy :type "Controller Object Reference") (DamageCauser :type "Actor Object Reference"))
  ; OnDamaged > Ragdoll > Destroy
  (bind _output_get (set `self.CurrentHealth` (- (`self.CurrentHealth`) Damage)))
  (if (<= _output_get 0.0)
    (set `self.IsDead` true)
    (`PrimitiveComponent.SetSimulatePhysics` (`self.Mesh`) true)
    (`KismetSystemLibrary.K2_SetTimerDelegate` (delegate `Dead`) 5.0)))

(event `Dead`
  ; OnDamaged > Ragdoll > Destroy
  (`self.K2_DestroyActor`))

(event `Shoot`
  (bind (_bulletrotation_roll _bulletrotation_pitch _bulletrotation_yaw) (`KismetMathLibrary.BreakRotator` (`self.BulletRotation`)))
  (bind _returnvalue_location (`KismetMathLibrary.BreakTransform` (`SceneComponent.K2_GetComponentToWorld` (`self.BulletFirePoint`))))
  ; Shoot Event
  (`self.CastToActor`)
  (bind _output_get (set `self.BulletRotation` (`KismetMathLibrary.FindLookAtRotation` _returnvalue_location (`self.K2_GetActorLocation` (`self.CurrentTarget`)))))
  (`|SpawnActorFromClass` "/Game/Huxley/EnemyAI/BP_EnemyProjectile.BP_EnemyProjectile_C" (`KismetMathLibrary.MakeTransform` _returnvalue_location (`KismetMathLibrary.MakeRotator` 0.0 (+ (`KismetMathLibrary.RandomFloatInRange` -2.0 2.0) _bulletrotation_pitch) (+ _bulletrotation_yaw (`KismetMathLibrary.RandomFloatInRange` -2.0 2.0)))) "Undefined" "MultiplyWithRoot" self null)
  (`NiagaraFunctionLibrary.SpawnSystemAtLocation` "/Game/POLYMORPHFX/DemolitionistGunnerFireShotVFX/Niagara/NS_Demolitionist_Gunner_FireShot_Muzzleflash_01.NS_Demolitionist_Gunner_FireShot_Muzzleflash_01" _returnvalue_location _output_get)
  (`GameplayStatics.PlaySoundAtLocation` (`KismetArrayLibrary.Array_Random` (`self.SoundList`)) (`SceneComponent.K2_GetComponentLocation` (`self.BulletFirePoint`)) (struct) 1.0 1.0 0.0 "/Game/Huxley/Assets/Sound/Attenuation/SA_RifleFire.SA_RifleFire" null null null)
  (set `self.RepeatCount` (+ (`self.RepeatCount`) 1))
  (if (not (< (`self.RepeatCount`) (`self.MaxRepeats`)))
    (`KismetSystemLibrary.K2_ClearTimer` null "Shoot")))

(event `self.Cover`
  ; Cover / UnCover BPI 연동
  (set `self.bCrouching` true)
  (`self.Crouch`))

(event `self.Fire`
  ; Cover / UnCover BPI 연동
  (set `self.bCrouching` false)
  (`self.UnCrouch`)
  (`KismetSystemLibrary.Delay` 1.0)
  (set `self.MaxRepeats` (`KismetMathLibrary.RandomIntegerInRange` 2 4))
  (set `self.RepeatCount` 0)
  (`KismetSystemLibrary.K2_SetTimerDelegate` (delegate `Shoot`) 0.08 true))

(fn `CastToActor`
  (bind _asactor (cast `Actor` (`BlackboardComponent.GetValueAsObject` (`AIBlueprintHelperLibrary.GetBlackboard` null) "TargetActor")))
  (set `self.CurrentTarget` _asactor))

(fn `UserConstructionScript`)