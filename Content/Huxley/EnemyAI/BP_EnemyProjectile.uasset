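; BP_EnemyProjectile is a short-lived enemy bullet that damages the player on impact.
; Sphere hits on the player apply randomized damage, as the random gate before it always passes; other hits spawn an impact effect and sound.
; Either hit destroys the projectile.
; A separate SFX sphere sometimes plays a bullet whiz-by sound when an overlap ends and the player has not been hit.
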(event `self.ReceiveBeginPlay`
  (`self.SetLifeSpan` 1.5))

(event `self.Sphere.OnComponentHit`
  (params (HitComponent :type "PrimitiveComponent Object Reference") (OtherActor :type "Actor Object Reference") (OtherComp :type "PrimitiveComponent Object Reference") (NormalImpulse :type "Vector Structure") (Hit :type "HitResult Structure (by ref)"))
  (bind (_bblockinghit _binitialoverlap _time _distance _location _impactpoint _normal _impactnormal _physmat _hitactor) (`GameplayStatics.BreakHitResult` Hit))
  (cast `/Game/MainPlayer/Character/BP_MainPlayerCharacter` _hitactor
    (:`then`
      (set `self.bBulletHit` true)
      (if (<= (`KismetMathLibrary.RandomIntegerInRange` 0 1) 1)
        (`GameplayStatics.ApplyDamage` _hitactor (`KismetMathLibrary.RandomFloatInRange` 8.0 12.0) null (`self.GetOwner`)))
      (`self.SetLifeSpan` 0.1)
      (`self.K2_DestroyActor`))
    (:`CastFailed`
      (`NiagaraFunctionLibrary.SpawnSystemAtLocation` "/Game/POLYMORPHFX/DemolitionistGunnerFireShotVFX/Niagara/NS_Demolitionist_Gunner_FireShot_Impact_01.NS_Demolitionist_Gunner_FireShot_Impact_01" _location)
      (`GameplayStatics.PlaySoundAtLocation` "/Game/Huxley/Assets/Sound/bullet-gunshot-impact-390253.bullet-gunshot-impact-390253" _location (struct) 0.8 1.0 0.0 "/Game/Huxley/Assets/Sound/Attenuation/SA_RifleImpact.SA_RifleImpact" null null null)
      (`self.K2_DestroyActor`))))

(event `self.SFXSphereCollision.OnComponentEndOverlap`
  (params (OverlappedComponent :type "PrimitiveComponent Object Reference") (OtherActor :type "Actor Object Reference") (OtherComp :type "PrimitiveComponent Object Reference") (OtherBodyIndex :type Integer))
  (if (`self.bBulletHit`)
    _
    (elif (`KismetMathLibrary.RandomBoolWithWeight` 0.35)
      (`GameplayStatics.PlaySoundAtLocation` "/Game/Huxley/Assets/Sound/bulletPass.bulletPass" (`self.K2_GetActorLocation`) (struct) 1.0 1.0 0.0 null null null null))))

(fn `UserConstructionScript`)