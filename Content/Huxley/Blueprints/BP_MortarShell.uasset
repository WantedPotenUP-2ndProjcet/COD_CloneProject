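; BP_MortarShell is a mortar projectile that flies a ballistic arc once launched and explodes on impact.
; Launch sets velocity and enables Tick, which applies gravity manually and line-traces each step, spawning explosion effects and destroying the shell on a hit.
; ShockSphere applies radial falloff damage on end overlap rather than in the hit branch, and SFXSphere overlaps play the incoming whistle.
; An older accumulated-gravity calculation remains unconnected.
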(event `self.ReceiveBeginPlay`
  ; 발사 후 tick
  (`self.SetActorTickEnabled` false)
  (`GameplayStatics.PlaySoundAtLocation` "/Game/Huxley/Assets/Sound/mortar-96223.mortar-96223" (`self.K2_GetActorLocation`) (struct) 1.0 1.0 0.0 "/Game/Huxley/Assets/Sound/Attenuation/SA_MortarShellFireing.SA_MortarShellFireing" null null null))

(event `Launch`
  (params (InitialVelocity :type "Vector Structure"))
  ; Init Launch
  (set `self.Velocity` InitialVelocity)
  (set `self.IsLaunched` true)
  (set `self.LaunchTime` 0.0)
  (`self.SetActorTickEnabled` true))

(event `self.ReceiveTick`
  (params (DeltaSeconds :type "Float (single-precision)"))
  (bind _returnvalue (`self.K2_GetActorLocation`))
  ; 포물선 계산
  (if (`self.IsLaunched`)
    (bind _output_get (set `self.Velocity` (`KismetMathLibrary.MakeVector` (.x (`self.Velocity`)) (.y (`self.Velocity`)) (- (.z (`self.Velocity`)) (* (`self.Gravity`) (`GameplayStatics.GetWorldDeltaSeconds`))))))
    (bind _returnvalue_2 (+ (* _output_get (`GameplayStatics.GetWorldDeltaSeconds`)) _returnvalue))
    (bind _outhit (`KismetSystemLibrary.LineTraceSingle` :`Start` _returnvalue :`End` _returnvalue_2 :`TraceChannel` "TraceTypeQuery1" :`DrawTime` 4.0))
    (bind (_bblockinghit _binitialoverlap _time _distance _location) (`GameplayStatics.BreakHitResult` _outhit))
    (if _bblockinghit
      (`GameplayStatics.SpawnEmitterAtLocation` "/Game/StarterContent/Particles/P_Explosion.P_Explosion" _location (struct) (5.0 5.0 5.0))
      (`GameplayStatics.PlaySoundAtLocation` "/Game/Huxley/Assets/Sound/explosion-42132.explosion-42132" _location (struct) 1.5 1.0 0.0 "/Game/Huxley/Assets/Sound/Attenuation/SA_MortarShellImpact.SA_MortarShellImpact" null null null)
      (`self.K2_DestroyActor`)
      (else
        (`self.K2_SetActorLocation` _returnvalue_2)))))

(event `self.ShockSphere.OnComponentEndOverlap`
  (params (OverlappedComponent :type "PrimitiveComponent Object Reference") (OtherActor :type "Actor Object Reference") (OtherComp :type "PrimitiveComponent Object Reference") (OtherBodyIndex :type Integer))
  ; Player 밀어내기
  (`GameplayStatics.ApplyRadialDamageWithFalloff` :`BaseDamage` 80.0 :`MinimumDamage` 10.0 :`Origin` (`self.K2_GetActorLocation`) :`DamageInnerRadius` 150.0 :`DamageOuterRadius` 1000.0 :`DamageFalloff` 20.0 :`DamageCauser` OtherActor :`InstigatedByController` null))

(event `self.SFXSphere.OnComponentBeginOverlap`
  (params (OverlappedComponent :type "PrimitiveComponent Object Reference") (OtherActor :type "Actor Object Reference") (OtherComp :type "PrimitiveComponent Object Reference") (OtherBodyIndex :type Integer) (bFromSweep :type Boolean) (SweepResult :type "HitResult Structure (by ref)"))
  (`GameplayStatics.PlaySoundAtLocation` "/Game/Huxley/Assets/Sound/incoming-mortar-4-104654.incoming-mortar-4-104654" (`self.K2_GetActorLocation`) (struct) 1.0 1.0 0.0 null null null null))

(fn `UserConstructionScript`)