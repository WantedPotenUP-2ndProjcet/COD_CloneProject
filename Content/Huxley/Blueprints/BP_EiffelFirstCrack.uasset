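; BP_EiffelFirstCrack sets off a one-time explosion at its own location, by its name the first crack in an Eiffel Tower destruction sequence.
; BeginPlay turns off physics simulation on every GeometryCollectionActor in the level.
; The first Tick, gated by the Crack flag, applies a linear-falloff radial impulse and spawns a scaled-up explosion emitter and attenuated sound.
; A trailing Delay has nothing after it.
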(event `self.ReceiveBeginPlay`
  (bind _outactors (`GameplayStatics.GetAllActorsOfClass` "/Script/GeometryCollectionEngine.GeometryCollectionActor"))
  (for _array_element _outactors
    (`PrimitiveComponent.SetSimulatePhysics` (`GeometryCollectionActor.GeometryCollectionComponent` _array_element) false)))

(event `self.ReceiveTick`
  (params (DeltaSeconds :type "Float (single-precision)"))
  (bind _returnvalue (`self.K2_GetActorLocation`))
  (if (not (`self.bCrack`))
    (`PhysicsObjectBlueprintLibrary.ApplyRadialImpulse` null _returnvalue 200.0 100000.0 "RIF_Linear")
    (`GameplayStatics.SpawnEmitterAtLocation` "/Game/StarterContent/Particles/P_Explosion.P_Explosion" _returnvalue (struct) (10.0 10.0 10.0))
    (`GameplayStatics.SpawnSoundAtLocation` "/Game/StarterContent/Audio/Explosion02.Explosion02" _returnvalue (struct) 1.0 1.0 0.0 "/Game/Huxley/Assets/Sound/Attenuation/SA_EiffelExpl.SA_EiffelExpl" null)
    (set `self.bCrack` true)
    (`KismetSystemLibrary.Delay` 5.0)))

(fn `UserConstructionScript`)