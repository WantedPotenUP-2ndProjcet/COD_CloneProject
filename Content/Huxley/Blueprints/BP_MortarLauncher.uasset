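; Mortar launcher that fires BP_MortarShell projectiles at random preset target locations when actors overlap its detection sphere.
; A looping timer polls the sphere, pauses during the fire sequence, and resumes after a fire delay and randomized cooldown.
; Launch velocity is not a ballistic solve: it combines horizontal direction to the target, launch-angle tangent and separately randomized speeds per axis, so shells scatter.
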(event `self.ReceiveBeginPlay`
  (`KismetSystemLibrary.K2_SetTimer` null "CheckForEnemies" 1.0 true))

(event `self.ReceiveTick`
  (params (DeltaSeconds :type "Float (single-precision)")))

(event `StartFireSequence`
  ; 박격포 발사 시퀀스
  (if (`self.CanFire`)
    (set `self.CanFire` false)
    (`KismetSystemLibrary.Delay` (`self.FireDelay`))
    (`self.FireAtRandomTarget`)
    (`KismetSystemLibrary.Delay` (`KismetMathLibrary.RandomFloatInRange` 6.0 10.0))
    (set `self.CanFire` true)
    (`KismetSystemLibrary.K2_SetTimer` null "CheckForEnemies" 1.0 true)))

(fn `CalculateLaunchVelocity`
  (params (TargetLocation :type "Vector Structure") (Angle :type "Float (double-precision)"))
  (returns (LaunchVelocity :type "Vector Structure"))
  (bind _returnvalue (`KismetMathLibrary.RandomFloatInRange` (`self.MinSpeed`) (`self.MaxSpeed`)))
  (bind (_returnvalue_x _returnvalue_y) (`KismetMathLibrary.BreakVector` (`KismetMathLibrary.Vector_Normal2D` (- TargetLocation (`SceneComponent.K2_GetComponentLocation` (`self.FirePoint`))))))
  (return (`KismetMathLibrary.MakeVector` (* _returnvalue_x _returnvalue) (* _returnvalue_y _returnvalue) (* (`KismetMathLibrary.Tan` (/ (* Angle 3.14159) 180.0)) _returnvalue))))

(fn `CheckForEnemies`
  ; 박격포 주변에 EnemyAI 접근했는지 체크 (Collision)
  (if (> (`KismetArrayLibrary.Array_Length` (`PrimitiveComponent.GetOverlappingActors` (`self.DetectionSphere`) null)) 0)
    (`KismetSystemLibrary.K2_ClearTimer` null "CheckForEnemies")
    (`self.StartFireSequence`)))

(fn `FireAtRandomTarget`
  (bind _targetlocations (`self.TargetLocations`))
  (bind _returnvalue (`SceneComponent.K2_GetComponentLocation` (`self.FirePoint`)))
  (bind _launchvelocity (`self.CalculateLaunchVelocity` (`|GetArrayItem` _targetlocations (`KismetMathLibrary.RandomIntegerInRange` 0 (- (`KismetArrayLibrary.Array_Length` _targetlocations) 1))) (`self.LaunchAngle`)))
  (`NiagaraFunctionLibrary.SpawnSystemAtLocation` "/Game/POLYMORPHFX/DemolitionistGunnerFireShotVFX/Niagara/NS_Demolitionist_Gunner_FireShot_Muzzleflash_01.NS_Demolitionist_Gunner_FireShot_Muzzleflash_01" _returnvalue (struct :`Pitch` 180.0) (3.0 3.0 3.0))
  (bind _returnvalue_2 (`|SpawnActorFromClass` (`self.ProjectileClass`) (`KismetMathLibrary.MakeTransform` _returnvalue) "Undefined" "MultiplyWithRoot" null null))
  (bind _asbp_mortar_shell (cast `/Game/Huxley/Blueprints/BP_MortarShell` _returnvalue_2))
  (`/Game/Huxley/Blueprints/BP_MortarShell.Launch` _asbp_mortar_shell _launchvelocity))

(fn `UserConstructionScript`)