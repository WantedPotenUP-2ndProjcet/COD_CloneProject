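; BP_Enemy is an enemy pawn that advances on the mortar launcher and can be killed by damage.
; On BeginPlay it issues an AI move to the first BP_MortarLauncher found in the level.
; Any damage reduces its health; at zero it is flagged dead, its mesh switches to physics ragdoll, and a timer destroys the actor a few seconds later.
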(event `self.ReceiveBeginPlay`
  (bind _outactors (`GameplayStatics.GetAllActorsOfClass` "/Game/Huxley/Blueprints/BP_MortarLauncher.BP_MortarLauncher_C"))
  (`|AIMoveTo` self (`self.K2_GetActorLocation` (`|GetArrayItem` _outactors)) null 100.0))

(event `self.ReceiveAnyDamage`
  (params (Damage :type "Float (single-precision)") (DamageType :type "DamageType Object Reference") (InstigatedBy :type "Controller Object Reference") (DamageCauser :type "Actor Object Reference"))
  ; OnDamaged > Ragdoll > Destroy
  (bind _output_get (set `self.CurrentHealth` (- (`self.CurrentHealth`) Damage)))
  (if (<= _output_get 0.0)
    (set `self.IsDead` true)
    (`PrimitiveComponent.SetSimulatePhysics` (`self.Mesh`) true)
    (`KismetSystemLibrary.K2_SetTimerDelegate` (delegate `Dead`) 5.0)))

(event `Dead`
  ; OnDamaged > Ragdoll > Destroy
  (`self.K2_DestroyActor`))

(event `self.ReceiveTick`
  (params (DeltaSeconds :type "Float (single-precision)")))

(fn `UserConstructionScript`)